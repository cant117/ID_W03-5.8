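; Player character for a 2D side-scroller with flipbook animation, Enhanced Input movement and jumping.
; CanMove gates both actions, while IsInfected turns movement input into paralysis with a dead flipbook and virus message.
; RespawnPlayer teleports to the location saved at BeginPlay and clears infection.
; The R key calls OpenLevel with LevelName None, passing the current level name as Options.
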(event `self.ReceiveBeginPlay`
  (bind _returnvalue (`InputDeviceLibrary.GetPlayerControllerFromInputDevice` (struct)))
  (`EnhancedInputSubsystemInterface.AddMappingContext` (pcsubsystem `EnhancedInputLocalPlayerSubsystem` _returnvalue) "/Game/Input/IMC_Player.IMC_Player" 0 (struct))
  (set `self.RespawnLocation` (`self.K2_GetActorLocation`)))

(event `EnhancedInput|/Game/Input/IA_Move`
  (params (ActionValue :type "Float (double-precision)") (ElapsedSeconds :type "Float (double-precision)") (TriggeredSeconds :type "Float (double-precision)") (InputAction :type "InputAction Object Reference" :default "/Game/Input/IA_Move.IA_Move"))
  (bind _isinfected (`self.IsInfected`))
  (bind _characterflipbook (`self.CharacterFlipbook`))
  (:`Triggered`
    (if (`self.CanMove`)
      (if _isinfected
        (`PaperFlipbookComponent.SetFlipbook` (`self.CharacterFlipbook`) "/Game/Textures/FB_Dead.FB_Dead")
        (`KismetSystemLibrary.PrintString` "病毒發作！肢體麻痺無法移動！" true true (struct :`R` 0.303125 :`A` 1.0))
        (else
          (`self.AddMovementInput` (1.0 0.0 0.0) ActionValue)
          (if (< ActionValue 0.0)
            (`SceneComponent.K2_SetRelativeRotation` _characterflipbook (struct :`Yaw` 180.0) false false)
            (else
              (`SceneComponent.K2_SetRelativeRotation` :`self` _characterflipbook)))
          (`PaperFlipbookComponent.SetFlipbook` (`self.CharacterFlipbook`) "/Game/Textures/FB_Walk.FB_Walk")))))
  (:`Completed`
    (if (not _isinfected)
      (`PaperFlipbookComponent.SetFlipbook` (`self.CharacterFlipbook`) "/Game/Textures/FB_Idle.FB_Idle"))))

(event `EnhancedInput|/Game/Input/IA_Jump`
  (params (ActionValue :type Boolean) (ElapsedSeconds :type "Float (double-precision)") (TriggeredSeconds :type "Float (double-precision)") (InputAction :type "InputAction Object Reference" :default "/Game/Input/IA_Jump.IA_Jump"))
  (:`Started`
    (if (`self.CanMove`)
      (`self.Jump`)
      (`PaperFlipbookComponent.SetFlipbook` (`self.CharacterFlipbook`) "/Game/Textures/FB_Jump.FB_Jump")
      (`KismetSystemLibrary.PrintString` "跳躍")))
  (:`Completed`
    (`self.StopJumping`)))

(event `RespawnPlayer`
  (`MovementComponent.StopMovementImmediately` (`self.CharacterMovement`))
  (`self.K2_SetActorLocation` (`self.RespawnLocation`) false true)
  (set `self.IsInfected` false)
  (`PaperFlipbookComponent.SetFlipbook` (`self.CharacterFlipbook`) "/Game/Textures/FB_Idle.FB_Idle")
  (`KismetSystemLibrary.PrintString` "角色已重生"))

(event `Key|R`
  (params (Key :type "Key Structure"))
  (:`Pressed`
    (bind _returnvalue (`GameplayStatics.GetCurrentLevelName` true))
    (`GameplayStatics.OpenLevel` "None" true _returnvalue)))

(fn `UserConstructionScript`)