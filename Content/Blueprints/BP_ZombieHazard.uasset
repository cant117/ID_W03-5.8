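; BP_ZombieHazard is a Paper2D zombie hazard that patrols along world X and infects the player on contact.
; A looping timer reverses its direction and flips the flipbook.
; Within DetectRange of the player, Tick sets IsChasing, which pauses turnarounds, and updates direction and actor rotation, but applies swept movement only outside that range.
; Box overlap sets the player's IsInfected flag and prints a warning.
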(event `self.ReceiveBeginPlay`
  (`KismetSystemLibrary.K2_SetTimerDelegate` (delegate `TurnAround`) 2.5 true))

(event `TurnAround`
  (bind _zb_flipbook (`self.ZB_Flipbook`))
  (if (not (`self.IsChasing`))
    (set `self.MoveDirection` (* (`self.MoveDirection`) -1.0))
    (if (> (`self.MoveDirection`) 0.0)
      (`SceneComponent.K2_SetRelativeRotation` :`self` _zb_flipbook)
      (else
        (`SceneComponent.K2_SetRelativeRotation` _zb_flipbook (struct :`Yaw` 180.0) false false)))))

(event `self.ReceiveTick`
  (params (DeltaSeconds :type "Float (single-precision)"))
  (bind _returnvalue (`GameplayStatics.GetPlayerCharacter` 0))
  (bind _x (.x (`self.K2_GetActorLocation` _returnvalue)))
  (if (< (`self.GetDistanceTo` _returnvalue null) (`self.DetectRange`))
    (set `self.IsChasing` true)
    (if (> (- _x (.x (- _x (`self.K2_GetActorLocation`)))) 0.0)
      (set `self.MoveDirection` 1.0)
      (`self.K2_SetActorRotation` (struct))
      (else
        (set `self.MoveDirection` -1.0)
        (`self.K2_SetActorRotation` (struct :`Yaw` 180.0))))
    (else
      (set `self.IsChasing` false)
      (`self.K2_AddActorWorldOffset` (`KismetMathLibrary.MakeVector` (* (* DeltaSeconds (`self.MoveSpeed`)) (`self.MoveDirection`))) true))))

(event `self.Box.OnComponentBeginOverlap`
  (params (OverlappedComponent :type "PrimitiveComponent Object Reference") (OtherActor :type "Actor Object Reference") (OtherComp :type "PrimitiveComponent Object Reference") (OtherBodyIndex :type Integer) (bFromSweep :type Boolean) (SweepResult :type "HitResult Structure (by ref)"))
  (bind _asbp_player_character (cast `/Game/Blueprints/BP_PlayerCharacter` OtherActor))
  (set `/Game/Blueprints/BP_PlayerCharacter.IsInfected` true _asbp_player_character)
  (`KismetSystemLibrary.PrintString` "遭到喪屍攻擊！已感染！" true true (struct :`R` 1.0 :`G` 0.26808 :`B` 0.142708 :`A` 1.0) 3.0))

(fn `UserConstructionScript`)