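; Parallax background actor that moves three layer components (far, mid, near) relative to the player camera along world X.
; Each Tick scales camera X by a per-layer factor, with the near layer matching it exactly, while every layer follows camera Z at its own fixed Y depth.
; The camera manager's player index comes from truncated DeltaSeconds, which is zero at sub-second frame times.
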(event `self.ReceiveBeginPlay`)

(event `self.ReceiveTick`
  (params (DeltaSeconds :type "Float (single-precision)"))
  (bind _x (.x (`self.K2_GetActorLocation` (`GameplayStatics.GetPlayerCameraManager` (`KismetMathLibrary.FTrunc` DeltaSeconds)))))
  (bind _z (.z (`self.K2_GetActorLocation` (`GameplayStatics.GetPlayerCameraManager` (`KismetMathLibrary.FTrunc` DeltaSeconds)))))
  (`SceneComponent.K2_SetWorldLocation` (`self.Layer_Far`) (`KismetMathLibrary.MakeVector` (* _x 0.9) -1500.0 _z) false false)
  (`SceneComponent.K2_SetWorldLocation` (`self.Layer_Mid`) (`KismetMathLibrary.MakeVector` (* _x 0.5) -600.0 _z) false false)
  (`SceneComponent.K2_SetWorldLocation` (`self.Layer_Near`) (`KismetMathLibrary.MakeVector` (* _x 1.0) 100.0 _z) false false))

(fn `UserConstructionScript`)