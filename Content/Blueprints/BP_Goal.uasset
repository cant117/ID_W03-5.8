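; BP_Goal is a level goal trigger that ends play with a victory screen when the player reaches it.
; Its Box overlap casts the other actor to BP_PlayerCharacter and sets IsCompleted so the sequence fires only once.
; It then adds WBP_Victory to the viewport, clears the player's CanMove, stops movement immediately and switches the character's flipbook to idle.
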(event `self.Box.OnComponentBeginOverlap`
  (params (OverlappedComponent :type "PrimitiveComponent Object Reference") (OtherActor :type "Actor Object Reference") (OtherComp :type "PrimitiveComponent Object Reference") (OtherBodyIndex :type Integer) (bFromSweep :type Boolean) (SweepResult :type "HitResult Structure (by ref)"))
  (if (not (`self.IsCompleted`))
    (bind _asbp_player_character (cast `/Game/Blueprints/BP_PlayerCharacter` OtherActor))
    (set `self.IsCompleted` true)
    (bind _returnvalue (`|CreateWidget` "/Game/WBP_Victory.WBP_Victory_C" (`GameplayStatics.GetPlayerController` 0)))
    (`UserWidget.AddToViewport` _returnvalue 0)
    (set `/Game/Blueprints/BP_PlayerCharacter.CanMove` false _asbp_player_character)
    (`MovementComponent.StopMovementImmediately` (`Character.CharacterMovement` _asbp_player_character))
    (`PaperFlipbookComponent.SetFlipbook` (`/Game/Blueprints/BP_PlayerCharacter.CharacterFlipbook` _asbp_player_character) "/Game/Textures/FB_Idle.FB_Idle")))

(fn `UserConstructionScript`)